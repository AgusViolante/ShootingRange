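; BP_Target is a shooting target that tips over when hit by a first-person projectile, awards points, then resets itself.
; A hit on the Sphere adds points scaled by Multiplier to the player character, then plays the drop.
; The DropTarget timeline lerps the Sphere from its starting rotation to a fixed dropped one, then reverses after ResetTime.
; The IsDown flag blocks scoring and repeat drops until the raise begins.
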(event `self.ReceiveBeginPlay`
  (set `self.Target Relative Rotation` (`SceneComponent.RelativeRotation` (`self.Sphere`))))

(event `self.Sphere.OnComponentHit`
  (params (HitComponent :type "PrimitiveComponent Object Reference") (OtherActor :type "Actor Object Reference") (OtherComp :type "PrimitiveComponent Object Reference") (NormalImpulse :type "Vector Structure") (Hit :type "HitResult Structure (by ref)"))
  (cast `/Game/FirstPerson/Blueprints/BP_FirstPersonProjectile` OtherActor)
  (`self.UpdateScore` 1)
  (`self.PlayTargetDrop`))

(event `PlayTargetDrop`
  (`TimelineComponent.SetPlayRate` (`self.DropTarget`) 1.0)
  (if (not (`self.IsDown`))
    (set `self.IsDown` true)
    (bind (_direction _rotatortarget) (`Timeline|DropTarget` :!label _label)
      (:`Update`
        (`SceneComponent.K2_SetRelativeRotation` (`self.Sphere`) (`KismetMathLibrary.RLerp` (`self.Target Relative Rotation`) (struct :`Pitch` -80.0) _rotatortarget) false false))
      (:`Finished`
        (if (`self.IsDown`)
          (`KismetSystemLibrary.Delay` (`self.ResetTime`))
          (`self.RaiseTarget`))))))

(event `RaiseTarget`
  (if (`self.IsDown`)
    (set `self.IsDown` false)
    (goto _label :!via `Reverse`)))

(fn `UpdateScore`
  (params (Score :type Integer))
  (if (not (`self.IsDown`))
    (bind _asbp_first_person_character (cast `/Game/FirstPerson/Blueprints/BP_FirstPersonCharacter` (`GameplayStatics.GetPlayerPawn` 0)))
    (`/Game/FirstPerson/Blueprints/BP_FirstPersonCharacter.ScoreAdd` _asbp_first_person_character (* Score (`self.Multiplier`)))))

(fn `UserConstructionScript`)