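; BP_MovingTarget is an actor whose sphere moves back and forth continuously between two points.
; On BeginPlay it caches the relative locations of the Sphere and the EndLocation component as endpoints.
; The MoveTarget timeline lerps the sphere between them, and its Finished output calls MovingTarget again, which flips IsForward to alternate Play and Reverse.
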(event `self.ReceiveBeginPlay`
  (`parent.ReceiveBeginPlay`)
  (set `self.Relative Location Start` (`SceneComponent.RelativeLocation` (`self.Sphere`)))
  (set `self.Relative Location End` (`SceneComponent.RelativeLocation` (`self.EndLocation`)))
  (`self.MovingTarget`))

(event `MovingTarget`
  (if (`self.IsForward`)
    (set `self.IsForward` false)
    (bind (_direction _alpha) (`Timeline|MoveTarget` :!label _label)
      (:`Update`
        (`SceneComponent.K2_SetRelativeLocation` (`self.Sphere`) (`KismetMathLibrary.VLerp` (`self.Relative Location Start`) (`self.Relative Location End`) _alpha) false false))
      (:`Finished`
        (`self.MovingTarget`)))
    (else
      (set `self.IsForward` true)
      (goto _label :!via `Reverse`))))

(fn `UserConstructionScript`
  (`parent.UserConstructionScript`))